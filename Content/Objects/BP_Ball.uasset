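; BP_Ball is a physics-driven ball that falls and displays its acceleration on screen, then removes itself.
; BeginPlay records the spawn time and gives the mesh a slight downward velocity.
; Tick prints vertical speed divided by time since spawn in m/s², an average rather than instantaneous acceleration.
; Once vertical velocity reads exactly zero, printing stops and a five-second timestamp countdown in Tick destroys the actor.
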(event EventBeginPlay
  (Variables|Default|SetTimeSpawn (Utilities|Time|GetTimeSeconds))
  (Physics|SetPhysicsLinearVelocity (Variables|Default|GetStaticMesh) "0.000000,0.000000,-1.000000" false "None"))

(event Collision|EventActorBeginOverlap
  (params (OtherActor :type Actor%20Object%20Reference)))

(event EventTick
  (params (DeltaSeconds :type Float%20%28single-precision%29))
  (if (not (Variables|Default|GetEsperandoADestruir))
    (Development|PrintText (Utilities|Text|FormatText "{aceleracion} m/s^2" (Utilities|Text|ToText(Float) (Math|Float|Absolute(Float) (Utilities|Operators|Divide (.z (Transformation|GetComponentVelocity (Variables|Default|GetStaticMesh))) (- (Utilities|Time|GetTimeSeconds) (Variables|Default|GetTimeSpawn)) 1e+02)) "HalfToEven" false true 1 324 0 2)) true false "(R=0.000000,G=0.660000,B=1.000000,A=1.000000)" 0.0)
    (if (== (.z (Transformation|GetComponentVelocity (Variables|Default|GetStaticMesh))) 0.0)
      (Variables|Default|SetTimer (+ (Utilities|Time|GetTimeSeconds) 5.0))
      (Variables|Default|SetEsperandoADestruir true))
    (elif (not (< (Utilities|Time|GetTimeSeconds) (Variables|Default|GetTimer)))
      (Actor|DestroyActor))))

(fn ConstructionScript)