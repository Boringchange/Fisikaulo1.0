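; BP_Frezbe is a physics-driven projectile actor that destroys the BP_Ardilla actor when it hits it.
; BeginPlay enables physics and, after a short delay, prints its X distance to the Ardilla.
; Interact sets the mesh velocity to NewVelocity and arms PermitDelete, letting StaticMeshActor hits destroy it.
; Tick destroys it through the DontExist flag, set by an Ardilla hit or by passing too far beyond the Ardilla along X.
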(event OnComponentHit(StaticMesh)
  (params (HitComponent :type Primitive%20Component%20Object%20Reference) (OtherActor :type Actor%20Object%20Reference) (OtherComp :type Primitive%20Component%20Object%20Reference) (NormalImpulse :type Vector :default "0, 0, 0") (Hit :type Hit%20Result%20Structure%20%28by%20ref%29))
  (if (== (Utilities|GetClass OtherActor) "/Game/Objects/Comitfail/BP_Ardilla.BP_Ardilla_C")
    (bind _returnvalue (Actor|GetActorOfClass "/Game/Objects/Comitfail/BP_Ardilla.BP_Ardilla_C"))
    (Actor|DestroyActor _returnvalue)
    (Variables|Default|SetDontExist true)
    (elif (Variables|Default|GetPermitDelete)
      (if (== (Utilities|GetClass OtherActor) "/Script/Engine.StaticMeshActor")
        (Actor|DestroyActor)))))

(event EventBeginPlay
  (Physics|SetSimulatePhysics (Variables|Default|GetStaticMesh) true)
  (Utilities|FlowControl|Delay 0.2)
  (bind _returnvalue (Actor|GetActorOfClass "/Game/Objects/Comitfail/BP_Ardilla.BP_Ardilla_C"))
  (Development|PrintText (Utilities|Text|FormatText "{distancia}m" (- (.x (Transformation|GetActorLocation _returnvalue)) (.x (Transformation|GetActorLocation))))))

(event Collision|EventActorBeginOverlap
  (params (OtherActor :type Actor%20Object%20Reference)))

(event EventTick
  (params (DeltaSeconds :type Float%20%28single-precision%29))
  (if (Variables|Default|GetDontExist)
    (Actor|DestroyActor)
    (else
      (bind _returnvalue (Actor|GetActorOfClass "/Game/Objects/Comitfail/BP_Ardilla.BP_Ardilla_C"))
      (if (> (.x (Transformation|GetWorldLocation (Variables|Default|GetStaticMesh))) (+ (.x (Transformation|GetActorLocation _returnvalue)) 3e+02))
        (Variables|Default|SetDontExist true)))))

(event EventInteract
  (params (NameObjectOfClassFreezbe :type Actor%20Object%20Reference))
  (Utilities|Casting|CastToBP_Frezbe NameObjectOfClassFreezbe)
  (Physics|SetPhysicsLinearVelocity (Variables|Default|GetStaticMesh) (Variables|Default|GetNewVelocity) false "None")
  (Variables|Default|SetPermitDelete true))

(event EventSendData
  (params (Velocity :type Vector :default "0, 0, 0")))

(fn ConstructionScript)